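; BP_Target is a lock-on target actor that reacts when a BP_FireBall hits it.
; At BeginPlay it caches the BP_Player found with GetActorOfClass.
; A fireball hit spawns an explosion at the impact point, switches the cube mesh to physics-only collision and hides its lock-on indicator.
; The same hit resets the player's lock-on flag and clears its fire target, while the actor itself stays in the level.
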(event EventBeginPlay
  (Variables|Default|SetLock%20on%20Indicator (Variables|Default|GetLockOnIndicator))
  (bind _returnvalue (Actor|GetActorOfClass "/Game/SS_LevelMap/Blueprints/BP_Player.BP_Player_C"))
  (Variables|Default|SetPlayer _returnvalue))

(event Collision|EventHit
  (params (MyComp :type Primitive%20Component%20Object%20Reference) (Other :type Actor%20Object%20Reference) (OtherComp :type Primitive%20Component%20Object%20Reference) (bSelfMoved :type Boolean) (HitLocation :type Vector :default "0, 0, 0") (HitNormal :type Vector :default "0, 0, 0") (NormalImpulse :type Vector :default "0, 0, 0") (Hit :type Hit%20Result%20Structure%20%28by%20ref%29))
  (Utilities|Casting|CastToBP_FireBall Other)
  (Variables|/Game/SS_LevelMap/Blueprints/BP_Player.BP_Player_C|SetIsLockOnComplate (Variables|Default|GetPlayer) false)
  (Effects|SpawnEmitteratLocation "/Game/Realistic_Starter_VFX_Pack_Vol2/Particles/Explosion/P_Explosion_Big_B.P_Explosion_Big_B" HitLocation "0, 0, 0" "3.000000,3.000000,3.000000")
  (Collision|SetCollisionEnabled (Variables|Default|Get1M_Cube_Chamfer1_DM) "PhysicsOnly")
  (Development|SetHiddeninGame (Variables|Default|GetLock%20on%20Indicator) true false)
  (Variables|/Game/SS_LevelMap/Blueprints/BP_Player.BP_Player_C|SetFireTarget (Variables|Default|GetPlayer) 0))

(fn ConstructionScript)