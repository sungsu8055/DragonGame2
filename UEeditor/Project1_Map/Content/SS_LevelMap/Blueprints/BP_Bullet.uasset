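; Homing bullet for the flying game that chases the player's fire target, captured at BeginPlay.
; Each tick it moves forward without sweep at its base speed plus the player's current forward speed, so the player cannot overtake it.
; While the target is valid, it lerps its rotation toward it with a changing weight, curving the path.
; On hit it spawns an explosion, clears the player's target, adds score and destroys itself.
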(event EventBeginPlay
  ;[1 1 1] 발사 속도 및 타겟 추적에 필요한 Class 가져오기
  (bind _returnvalue (Actor|GetActorOfClass "/Game/SS_LevelMap/Blueprints/BP_Player.BP_Player_C"))
  (bind _output_get (Variables|Default|SetPlayer _returnvalue))
  (Variables|Default|SetTarget (Variables|/Game/SS_LevelMap/Blueprints/BP_Player.BP_Player_C|GetFireTarget _output_get))
  (bind _returnvalue_2 (Actor|GetActorOfClass "/Game/SS_LevelMap/Blueprints/FlyingGameMode.FlyingGameMode_C"))
  (Variables|Default|SetFlyingGameMode _returnvalue_2))

(event EventTick
  (params (DeltaSeconds :type Float%20%28single-precision%29))
  ;[1 1 1] 추적 함수에 발사속도 및 이동 방향 제공
  (bind _fireattackspeed (CallFunction|CalculateFireSpeed))
  ;[1 1 1] 추적 기능 실행
  (CallFunction|TrackingTarget (Transformation|GetActorForwardVector) DeltaSeconds _fireattackspeed (Variables|Default|GetTarget)))

(event Collision|EventHit
  (params (MyComp :type Primitive%20Component%20Object%20Reference) (Other :type Actor%20Object%20Reference) (OtherComp :type Primitive%20Component%20Object%20Reference) (bSelfMoved :type Boolean) (HitLocation :type Vector :default "0, 0, 0") (HitNormal :type Vector :default "0, 0, 0") (NormalImpulse :type Vector :default "0, 0, 0") (Hit :type Hit%20Result%20Structure%20%28by%20ref%29))
  ;[1 1 1] 타겟과 충돌 시 이펙트 출력과 함께 서로 파괴
  (Effects|SpawnEmitteratLocation "/Game/StarterContent/Particles/P_Explosion.P_Explosion" (Transformation|GetActorLocation) "0, 0, 0" "5.000000,5.000000,5.000000")
  (Variables|/Game/SS_LevelMap/Blueprints/BP_Player.BP_Player_C|SetFireTarget (Variables|Default|GetPlayer) 0)
  (Default|AddScore (Variables|Default|GetFlyingGameMode))
  (Actor|DestroyActor))

(fn ConstructionScript)

(fn TrackingTarget
  (params (Direction :type Vector) (DeltaTime :type Float%20%28single-precision%29) (Speed :type Float%20%28single-precision%29) (Target :type Actor%20Object%20Reference))
  ;[1 1 1] forward 방향으로만 지속 이동
  (Transformation|SetActorLocation (+ (Transformation|GetActorLocation) (* (* (Math|Vector|Normalize Direction) Speed) DeltaTime)) false false)
  (Utilities|IsValid Target
    (:Is%20Valid
      (bind _output_get (Variables|Default|SetTrackingLerpRatio (Math|Float|Lerp (Variables|Default|GetTrackingLerpRatio) 25.0 (Variables|Default|GetWeight))))
      (bind _output_get_2 (Variables|Default|SetWeight (* _output_get (Utilities|Time|GetWorldDeltaSeconds))))
      ;[1 1 1] forward 방향이 점점 타겟을 바라보게 되어 추적하는 효과 발생
      (Transformation|SetActorRotation (Math|Rotator|Lerp(Rotator) (Transformation|GetActorRotation) (Math|Rotator|FindLookatRotation (Transformation|GetActorLocation) (Transformation|GetActorLocation Target)) _output_get_2)))))

(fn CalculateFireSpeed
  (return (+ (Variables|Default|GetBulletSpeed) (Variables|/Game/SS_LevelMap/Blueprints/BP_Player.BP_Player_C|GetCurrent%20forward%20speed (Variables|Default|GetPlayer)))))