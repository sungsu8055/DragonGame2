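; FlyingGameMode is the game mode for a flying, target-based score level.
; On BeginPlay it caches a boost trigger and a target actor, then adds the points and HP bar widgets to the viewport.
; AddScore raises the current score, and Tick keeps BestScore at the highest value reached.
; Tick also calls GameOver, which checks for remaining targets but does nothing, as its game-over print is disconnected.
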(event EventBeginPlay
  (bind _returnvalue (Actor|GetActorOfClass "/Game/SS_LevelMap/Blueprints/BP_BoostModeTrigger.BP_BoostModeTrigger_C"))
  (Variables|Default|SetBoostZone _returnvalue)
  (bind _returnvalue_2 (Actor|GetActorOfClass "/Game/SS_LevelMap/Blueprints/BP_Target.BP_Target_C"))
  (Variables|Default|SetTarget _returnvalue_2)
  (bind _returnvalue_3 (UserInterface|CreateWidget "/Game/SS_LevelMap/Blueprints/WBP_Points.WBP_Points_C"))
  (bind _output_get (Variables|Default|SetHUD _returnvalue_3))
  (UserInterface|Viewport|AddtoViewport _output_get 0)
  (bind _returnvalue_4 (UserInterface|CreateWidget "/Game/SS_LevelMap/Blueprints/WBP_HPBar.WBP_HPBar_C"))
  (UserInterface|Viewport|AddtoViewport _returnvalue_4 0))

(event EventTick
  (params (DeltaSeconds :type Float%20%28single-precision%29))
  (bind _currentscore (Variables|Default|GetCurrentScore))
  (CallFunction|GameOver)
  (if (> _currentscore (Variables|Default|GetBestScore))
    (Variables|Default|SetBestScore _currentscore)))

(fn ConstructionScript)

(fn AddScore
  (params (RedZone :type Integer))
  (Variables|Default|SetCurrentScore (+ (Variables|Default|GetCurrentScore) RedZone)))

(fn GameOver
  (bind _outactors (Actor|GetAllActorsOfClass "/Game/SS_LevelMap/Blueprints/BP_Target.BP_Target_C"))
  (bind _output_get (Variables|Default|SetOut%20Actors _outactors))
  (if (<= (Utilities|Array|Length _output_get) 0)
    _))