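; BP_FireBall is a homing projectile that chases the player's fire target in the flying level.
; Each tick it moves forward at bullet speed plus the player's forward speed, lerps its rotation toward the target with growing weight, and billboards its fire effect to the camera.
; Hitting BP_Target or BP_TargetTower applies impulse and radial damage, scoring only for BP_Target.
; Those hits and any overlap spawn explosion effects, clear the player's target and destroy it.
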(event EventBeginPlay
  ;[1 1 1] 발사 속도 및 타겟 추적에 필요한 Class 가져오기
  (bind _returnvalue (Actor|GetActorOfClass "/Game/SS_LevelMap/Blueprints/BP_Player.BP_Player_C"))
  (bind _output_get (Variables|Default|SetPlayer _returnvalue))
  (bind _asbp_target (Utilities|Casting|CastToBP_Target (Variables|/Game/SS_LevelMap/Blueprints/BP_Player.BP_Player_C|GetFireTarget _output_get)))
  (Variables|Default|SetTarget _asbp_target)
  (bind _returnvalue_2 (Actor|GetActorOfClass "/Game/SS_LevelMap/Blueprints/FlyingGameMode.FlyingGameMode_C"))
  (Variables|Default|SetFlyingGameMode _returnvalue_2))

(event Collision|EventActorBeginOverlap
  (params (OtherActor :type Actor%20Object%20Reference))
  (bind _returnvalue (Transformation|GetActorLocation))
  (Effects|SpawnEmitteratLocation "/Game/Realistic_Starter_VFX_Pack_Vol2/Particles/Explosion/P_Explosion_Big_A.P_Explosion_Big_A" _returnvalue "0, 0, 0" "2.000000,2.000000,2.000000")
  (Effects|SpawnEmitteratLocation "/Game/Realistic_Starter_VFX_Pack_Vol2/Particles/Sparks/P_Sparks_G.P_Sparks_G" _returnvalue "0, 0, 0" "3.000000,3.000000,3.000000")
  (Variables|/Game/SS_LevelMap/Blueprints/BP_Player.BP_Player_C|SetFireTarget (Variables|Default|GetPlayer) 0)
  (Effects|SpawnEmitteratLocation "/Game/Realistic_Starter_VFX_Pack_Vol2/Particles/Fire/P_Fire_Small.P_Fire_Small" _returnvalue "0, 0, 0" "2.000000,2.000000,2.000000")
  (Actor|DestroyActor))

(event EventTick
  (params (DeltaSeconds :type Float%20%28single-precision%29))
  ;[1 1 1] 추적 함수에 발사속도 및 이동 방향 제공
  (bind _fireattackspeed (CallFunction|CalculateFireSpeed))
  ;[1 1 1] 추적 기능 실행
  (CallFunction|TrackingTarget (Transformation|GetActorForwardVector) DeltaSeconds _fireattackspeed (Variables|Default|GetTarget))
  (CallFunction|FireBallBillboard))

(event Collision|EventHit
  (params (MyComp :type Primitive%20Component%20Object%20Reference) (Other :type Actor%20Object%20Reference) (OtherComp :type Primitive%20Component%20Object%20Reference) (bSelfMoved :type Boolean) (HitLocation :type Vector :default "0, 0, 0") (HitNormal :type Vector :default "0, 0, 0") (NormalImpulse :type Vector :default "0, 0, 0") (Hit :type Hit%20Result%20Structure%20%28by%20ref%29))
  (bind _returnvalue (Transformation|GetActorLocation))
  (bind _returnvalue_2 (Transformation|GetActorLocation))
  ;[1 1 1] 타겟과 충돌 시 이펙트 출력과 함께 서로 파괴
  (Utilities|FlowControl|Sequence
    (:then_0
      (bind _asbp_target (Utilities|Casting|CastToBP_Target Other))
      (Physics|AddImpulseatLocation OtherComp (* (Transformation|GetVelocity) 1e+02) _returnvalue_2 "None")
      (Class|DestructibleComponent|ApplyRadiusDamage (Variables|/Game/SS_LevelMap/Blueprints/BP_Target.BP_Target_C|Get1M_Cube_Chamfer1_DM _asbp_target) 1e+03 _returnvalue_2 5e+03 1.05e+05 false)
      (Default|AddScore (Variables|Default|GetFlyingGameMode) 2))
    (:then_1
      (bind _asbp_target_tower (Utilities|Casting|CastToBP_TargetTower Other))
      (Physics|AddImpulseatLocation OtherComp (* (Transformation|GetVelocity) 1e+02) _returnvalue "None")
      (Class|DestructibleComponent|ApplyRadiusDamage (Variables|/Game/SS_LevelMap/Blueprints/BP_TargetTower.BP_TargetTower_C|GetTargetTower _asbp_target_tower) 1e+03 _returnvalue 1.9e+03 1e+04 false)))
  (Effects|SpawnEmitteratLocation "/Game/Realistic_Starter_VFX_Pack_Vol2/Particles/Explosion/P_Explosion_Big_A.P_Explosion_Big_A" HitLocation "0, 0, 0" "5.000000,5.000000,5.000000")
  (Effects|SpawnEmitteratLocation "/Game/Realistic_Starter_VFX_Pack_Vol2/Particles/Sparks/P_Sparks_G.P_Sparks_G" HitLocation (Math|Conversions|RotationFromXVector HitNormal) "5.000000,5.000000,5.000000")
  (Variables|/Game/SS_LevelMap/Blueprints/BP_Player.BP_Player_C|SetFireTarget (Variables|Default|GetPlayer) 0)
  (Actor|DestroyActor))

(fn ConstructionScript)

(fn TrackingTarget
  (params (Direction :type Vector) (DeltaTime :type Float%20%28single-precision%29) (Speed :type Float%20%28single-precision%29) (Target :type Actor%20Object%20Reference))
  ;[1 1 1] forward 방향으로만 지속 이동
  (Transformation|SetActorLocation (+ (Transformation|GetActorLocation) (* (* (Math|Vector|Normalize Direction) Speed) DeltaTime)) true false)
  (Utilities|IsValid Target
    (:Is%20Valid
      (bind _output_get (Variables|Default|SetTrackingLerpRatio (Math|Float|Lerp (Variables|Default|GetTrackingLerpRatio) 25.0 (Variables|Default|GetWeight))))
      (bind _output_get_2 (Variables|Default|SetWeight (* _output_get (Utilities|Time|GetWorldDeltaSeconds))))
      ;[1 1 1] forward 방향이 점점 타겟을 바라보게 되어 추적하는 효과 발생
      (Transformation|SetActorRotation (Math|Rotator|Lerp(Rotator) (Transformation|GetActorRotation) (Math|Rotator|FindLookatRotation (Transformation|GetActorLocation) (Transformation|GetActorLocation Target)) _output_get_2 true)))))

(fn CalculateFireSpeed
  (return (+ (Variables|Default|GetBulletSpeed) (Variables|/Game/SS_LevelMap/Blueprints/BP_Player.BP_Player_C|GetCurrent%20forward%20speed (Variables|Default|GetPlayer)))))

(fn FireBallBillboard
  (bind _returnvalue (Game|GetPlayerCameraManager 0))
  (bind _returnvalue_2 (Transformation|GetActorLocation))
  (bind _returnvalue_3 (Camera|GetCameraLocation _returnvalue))
  (bind _returnvalue_4 (- _returnvalue_3 _returnvalue_2))
  (bind _returnvalue_5 (Math|Vector|Normalize _returnvalue_4))
  (bind _returnvalue_6 (Math|Conversions|RotationFromXVector _returnvalue_5))
  (Utilities|IsValid (Variables|Default|GetFireEffect)
    (:Is%20Valid
      (Transformation|SetWorldRotation (Variables|Default|GetFireEffect) (Math|Rotator|MakeRotator (.roll _returnvalue_6) (+ (.pitch _returnvalue_6) -9e+01) (.yaw _returnvalue_6)) false false))))