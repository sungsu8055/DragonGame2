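; Projectile actor that flies toward a point ahead of the player, presumably fired by BP_Target enemies.
; On BeginPlay it gets the player from the first BP_Target found and sets a one-time direction toward a fixed lead point along FirePosition1's forward vector.
; Tick moves it along that direction at constant speed with a swept SetActorLocation and billboards FireEffect toward the camera with a pitch offset.
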(event EventBeginPlay
  (bind _returnvalue (Actor|GetActorOfClass "/Game/SS_LevelMap/Blueprints/BP_Target.BP_Target_C"))
  (bind _asbp_player (Utilities|Casting|CastToBP_Player (Variables|/Game/SS_LevelMap/Blueprints/BP_Target.BP_Target_C|GetTargetPlayer _returnvalue)))
  (CallFunction|PredictiveShooting _asbp_player))

(event Collision|EventActorBeginOverlap
  (params (OtherActor :type Actor%20Object%20Reference)))

(event EventTick
  (params (DeltaSeconds :type Float%20%28single-precision%29))
  (CallFunction|Shoot (Variables|Default|GetTargetDir) 1.2e+04 DeltaSeconds)
  (CallFunction|FireBallBillboard))

(fn ConstructionScript)

(fn FireBallBillboard
  (bind _returnvalue (Game|GetPlayerCameraManager 0))
  (bind _returnvalue_2 (Transformation|GetActorLocation))
  (bind _returnvalue_3 (Camera|GetCameraLocation _returnvalue))
  (bind _returnvalue_4 (- _returnvalue_3 _returnvalue_2))
  (bind _returnvalue_5 (Math|Vector|Normalize _returnvalue_4))
  (bind _returnvalue_6 (Math|Conversions|RotationFromXVector _returnvalue_5))
  (Utilities|IsValid (Variables|Default|GetFireEffect)
    (:Is%20Valid
      (Transformation|SetWorldRotation (Variables|Default|GetFireEffect) (Math|Rotator|MakeRotator (.roll _returnvalue_6) (+ (.pitch _returnvalue_6) -9e+01) (.yaw _returnvalue_6)) false false))))

(fn PredictiveShooting
  (params (TG :type BP%20Player%20Object%20Reference))
  (bind _fireposition1 (Variables|/Game/SS_LevelMap/Blueprints/BP_Player.BP_Player_C|GetFirePosition1 TG))
  (Variables|Default|SetTargetDir (- (+ (Transformation|GetWorldLocation _fireposition1) (* (Math|Vector|GetForwardVector _fireposition1) 3e+03)) (Transformation|GetActorLocation))))

(fn Shoot
  (params (Dir :type Vector) (Speed :type Float%20%28single-precision%29) (Delta :type Float%20%28single-precision%29))
  ;[1 1 1] forward 방향으로만 지속 이동
  (Transformation|SetActorLocation (+ (Transformation|GetActorLocation) (* (* (Math|Vector|Normalize Dir) Speed) Delta)) true false))